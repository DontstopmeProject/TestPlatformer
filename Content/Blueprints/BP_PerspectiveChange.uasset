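; Door that switches the player pawn between In and Out perspectives when F is pressed, with prompt text shown on overlap.
; The sequence disables input, swings the door open, teleports the pawn to the side's target actor, then closes the door and restores input.
; A timeline rotates the pawn and any held object toward the new orientation and applies that side's physics constraint mode before the In state flips.
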(event `OpenTheDoor`
  (params (Reverse :type Boolean))
  (if Reverse
    (bind (_direction _newtrack_0) (`Timeline|DoorOpenTimeline` :!via `ReverseFromEnd` :!label _label)
      (:`Update`
        (`SceneComponent.K2_SetRelativeRotation` (`self.Capsule`) (`KismetMathLibrary.MakeRotator` 0.0 0.0 (select `bool` (`self.in`) :`false` _newtrack_0 :`true` (* _newtrack_0 -1.0))) false false)))
    (else
      (goto _label :!via `PlayFromStart`))))

(event `/Game/Blueprints/Interfaces/BPI_Keys.KeyPressed`
  (params (`Key ` :type "Key Structure"))
  (if (== `Key ` "F")
    (`self.EventChangePerspective`)))

(event `EventChangePerspective`
  (bind _returnvalue (select `bool` (`self.in`) :`false` (`self.OutConstraintMode`) :`true` (`self.InConstraintMode`)))
  (if (not (`self.Opening`))
    (if (`self.in`)
      (`SceneComponent.SetVisibility` (`self.TextRenderIn`) false false)
      (else
        (`SceneComponent.SetVisibility` (`self.TextRenderOut`) false false)))
    (set `self.Opening` true)
    (`self.DisableInput` (`self.OverlappedPawn`) (`GameplayStatics.GetPlayerController` 0))
    (`PrimitiveComponent.SetSimulatePhysics` (`/Game/SideScrollerBP/Blueprints/BP_TestPawn.Capsule` (`self.OverlappedPawn`)) false)
    (`self.OpenTheDoor` false)
    (`KismetSystemLibrary.Delay` 2.2)
    (`PrimitiveComponent.SetSimulatePhysics` (`/Game/SideScrollerBP/Blueprints/BP_TestPawn.Capsule` (`self.OverlappedPawn`)) true)
    (`PrimitiveComponent.SetConstraintMode` (`/Game/SideScrollerBP/Blueprints/BP_TestPawn.Capsule` (`self.OverlappedPawn`)) "SixDOF")
    (`self.K2_SetActorLocation` (`self.OverlappedPawn`) (`self.K2_GetActorLocation` (`|GetArrayItem` (`self.TeleportActor`) (select `bool` (`self.in`) :`false` 1))) false false)
    (`KismetSystemLibrary.Delay` 1.0)
    (bind (_direction _newtrack_0) (`Timeline|Timeline_0` :!via `PlayFromStart`)
      (:`Update`
        (bind _returnvalue_2 (`KismetMathLibrary.RInterpTo_Constant` (`SceneComponent.K2_GetComponentRotation` (`/Game/SideScrollerBP/Blueprints/BP_TestPawn.Capsule` (`self.OverlappedPawn`))) (select `bool` (`self.in`) :`false` (`self.OutTargetRotation`) :`true` (`self.InTargetRotation`)) _newtrack_0 10.0))
        (`SceneComponent.K2_SetWorldRotation` (`/Game/SideScrollerBP/Blueprints/BP_TestPawn.Capsule` (`self.OverlappedPawn`)) _returnvalue_2 false false)
        (`PrimitiveComponent.SetConstraintMode` (`/Game/SideScrollerBP/Blueprints/BP_TestPawn.Capsule` (`self.OverlappedPawn`)) _returnvalue)
        (if (`KismetSystemLibrary.IsValid` (`/Game/Blueprints/Components/GrabObjetcsComponent.HoldingComponent` (`self.GrabObjectsComponent`)))
          (`SceneComponent.K2_SetWorldRotation` (`/Game/Blueprints/Components/GrabObjetcsComponent.HoldingComponent` (`self.GrabObjectsComponent`)) _returnvalue_2 false false)
          (`PrimitiveComponent.SetConstraintMode` (`/Game/Blueprints/Components/GrabObjetcsComponent.HoldingComponent` (`self.GrabObjectsComponent`)) _returnvalue)))
      (:`Finished`
        (`self.OpenTheDoor` true)
        (`KismetSystemLibrary.Delay` 3.0)
        (if (`self.in`)
          (set `self.in` false)
          (else
            (set `self.in` true)))
        (`self.EnableInput` (`self.OverlappedPawn`) (`GameplayStatics.GetPlayerController` 0))
        (set `self.Opening` false)
        (if (`self.in`)
          (`SceneComponent.SetVisibility` (`self.TextRenderIn`) true false)
          (else
            (`SceneComponent.SetVisibility` (`self.TextRenderOut`) true false)))))))

(event `self.Box.OnComponentBeginOverlap`
  (params (OverlappedComponent :type "PrimitiveComponent Object Reference") (OtherActor :type "Actor Object Reference") (OtherComp :type "PrimitiveComponent Object Reference") (OtherBodyIndex :type Integer) (bFromSweep :type Boolean) (SweepResult :type "HitResult Structure (by ref)"))
  (bind (_asbp_test_pawn _bsuccess) (cast `/Game/SideScrollerBP/Blueprints/BP_TestPawn` OtherActor :!pure true))
  (if _bsuccess
    (set `self.OverlappedPawn` _asbp_test_pawn)
    (set `self.GrabObjectsComponent` (`/Game/SideScrollerBP/Blueprints/ZeroGravityController.GrabObjetcsComponent` (cast `/Game/SideScrollerBP/Blueprints/ZeroGravityController` (`Pawn.GetController` (`self.OverlappedPawn`)) :!pure true)))
    (if (`self.in`)
      (`SceneComponent.SetVisibility` (`self.TextRenderIn`) true false)
      (else
        (`SceneComponent.SetVisibility` (`self.TextRenderOut`) true false)))))

(event `self.Box.OnComponentEndOverlap`
  (params (OverlappedComponent :type "PrimitiveComponent Object Reference") (OtherActor :type "Actor Object Reference") (OtherComp :type "PrimitiveComponent Object Reference") (OtherBodyIndex :type Integer))
  (if (`self.in`)
    (`SceneComponent.SetVisibility` (`self.TextRenderIn`) false false)
    (else
      (`SceneComponent.SetVisibility` (`self.TextRenderOut`) false false))))

(fn `UserConstructionScript`)