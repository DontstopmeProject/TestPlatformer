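; An actor component, owned by the ZeroGravityController, that lets the controlled BP_TestPawn grab and release physics objects.
; EventToggleGrab either releases the held object or grabs the pawn's attached overlapped component through its PhysicsHandle at the AttachSphere location, tracking what is held.
; Tick moves the handle's target to the AttachSphere every frame, so a held object follows the pawn.
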(event `EventToggleGrab`
  (bind _player_spawn (`self.Player'sPawn`))
  (if (`self.HoldsActor`)
    (`PhysicsHandleComponent.ReleaseComponent` (`/Game/SideScrollerBP/Blueprints/BP_TestPawn.PhysicsHandle` (`self.Player'sPawn`)))
    (set `self.HoldsActor` false)
    (set `self.HoldingActor` null)
    (set `self.HoldingComponent` null)
    (`KismetSystemLibrary.PrintString` "Detached")
    (elif (`KismetSystemLibrary.IsValid` (`/Game/SideScrollerBP/Blueprints/BP_TestPawn.AttachedOverlappedActor` (`self.Player'sPawn`)))
      (`|ExecutionSequence`
        (:`then_0`
          (set `self.HoldingActor` (`/Game/SideScrollerBP/Blueprints/BP_TestPawn.AttachedOverlappedActor` (`self.Player'sPawn`)))
          (set `self.HoldsActor` true)
          (set `self.HoldingComponent` (`/Game/SideScrollerBP/Blueprints/BP_TestPawn.AttachedOverlappedComponent` (`self.Player'sPawn`)))
          (`KismetSystemLibrary.PrintString` "Attached"))
        (:`then_1`
          (`PhysicsHandleComponent.GrabComponentAtLocation` (`/Game/SideScrollerBP/Blueprints/BP_TestPawn.PhysicsHandle` _player_spawn) (`self.HoldingComponent`) "None" (`SceneComponent.K2_GetComponentLocation` (`/Game/SideScrollerBP/Blueprints/BP_TestPawn.AttachSphere` _player_spawn)))))
      (else
        (set `self.HoldsActor` false)))))

(event `self.ReceiveBeginPlay`
  (set `self.Player'sPawn` (cast `/Game/SideScrollerBP/Blueprints/BP_TestPawn` (`Controller.K2_GetPawn` (cast `/Game/SideScrollerBP/Blueprints/ZeroGravityController` (`self.GetOwner`) :!pure true)) :!pure true)))

(event `self.ReceiveTick`
  (params (DeltaSeconds :type "Float (single-precision)"))
  (`PhysicsHandleComponent.SetTargetLocation` (`/Game/SideScrollerBP/Blueprints/BP_TestPawn.PhysicsHandle` (`self.Player'sPawn`)) (`SceneComponent.K2_GetComponentLocation` (`/Game/SideScrollerBP/Blueprints/BP_TestPawn.AttachSphere` (`self.Player'sPawn`)))))